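; BP_ScorePickUp is a collectible actor that adds points to the player's score.
; On BeginPlay it casts and caches a reference to BP_GameInstance.
; When its collider overlaps a BP_Player, it adds its per-instance ScoreValue to the Game Instance's CurrentScore, then destroys itself.
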(event OnComponentBeginOverlap(Collider)
  (params (OverlappedComponent :type Primitive%20Component%20Object%20Reference) (OtherActor :type Actor%20Object%20Reference) (OtherComp :type Primitive%20Component%20Object%20Reference) (OtherBodyIndex :type Integer) (bFromSweep :type Boolean) (SweepResult :type Hit%20Result%20Structure%20%28by%20ref%29))
  (bind _gameinstance (Variables|Default|GetGameInstance))
  ;[0.03119 1 0.1322 0.5] When this collider overlaps, we check to see if it was the Player, and if so, set the value of CurrentScore on the Game Instance to be CurrentScore + ScoreValue (the value of this instance of the BP_ScorePickUp), then destroy this actor.
  (Utilities|Casting|CastToBP_Player OtherActor)
  (Variables|/Game/BlockHead/Core/Game/BP_GameInstance.BP_GameInstance_C|SetCurrentScore _gameinstance (+ (Variables|Default|GetScoreValue) (Variables|/Game/BlockHead/Core/Game/BP_GameInstance.BP_GameInstance_C|GetCurrentScore _gameinstance)))
  (Actor|DestroyActor))

(event EventBeginPlay
  ;[0.03119 1 0.1322 0.5] Store a reference to the Game Instance
  (bind _asbp_game_instance (Utilities|Casting|CastToBP_GameInstance (Game|GetGameInstance)))
  (Variables|Default|SetGameInstance _asbp_game_instance))

(fn ConstructionScript)